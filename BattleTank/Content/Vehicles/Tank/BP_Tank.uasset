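; Player-controllable tank that wires its components together and maps input to driving, camera aiming and firing.
; BeginPlay hands the barrel, turret and hull to the aiming component, and both tracks to the movement component.
; Aim axes rotate an azimuth gimbal and spring arm, scaled by delta time; drive input either sets each track's throttle or sends move/turn intent to TankMovement.
; Force-feedback and extra throttle nodes are disconnected and never run.
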(event `self.ReceiveBeginPlay`
  (`TankAimingComponent.InitialiseAiming` (`self.TankAimingAITank`) (`self.Barrel`) (`self.Turret`) (`self.TankHull`))
  (`TankMovementComponent.Initialise` (`self.TankMovement`) (`self.LeftTrack`) (`self.RightTrack`)))

(event `InputAxis|AimAzimuth`
  (params (AxisValue :type "Float (single-precision)"))
  ;[1 1 1] Camera Input Binding
  ;;[1 1 1] X Axis
  (`SceneComponent.K2_AddLocalRotation` (`self.Azimuth Gimbal`) (`KismetMathLibrary.MakeRotator` 0.0 0.0 (* AxisValue (`GameplayStatics.GetWorldDeltaSeconds`) 100.0)) false false))

(event `InputAction|Fire`
  (params (Key :type "Key Structure"))
  ;[1 1 1] Action Input Binding
  ;;[1 1 1] Fire
  (:`Pressed`
    (`TankAimingComponent.Fire` (`self.TankAimingAITank`))))

(event `InputAxis|Right Track Throttle`
  (params (AxisValue :type "Float (single-precision)"))
  ;[1 1 1] Action Input Binding
  (`TankTrack.SetThrottle` (`self.RightTrack`) AxisValue))

(event `InputAxis|Left Track Throttle`
  (params (AxisValue :type "Float (single-precision)"))
  ;[1 1 1] Action Input Binding
  (`TankTrack.SetThrottle` (`self.LeftTrack`) AxisValue))

(event `InputAxis|AimElevation`
  (params (AxisValue :type "Float (single-precision)"))
  ;[1 1 1] Camera Input Binding
  ;;[1 1 1] Y Axis
  (`SceneComponent.K2_AddLocalRotation` (`self.SpringArm`) (`KismetMathLibrary.MakeRotator` 0.0 (* AxisValue (`GameplayStatics.GetWorldDeltaSeconds`) 100.0)) false false))

(event `InputAxis|Move`
  (params (AxisValue :type "Float (single-precision)"))
  ;[1 1 1] Action Input Binding
  (`TankMovementComponent.IntendMoveForward` (`self.TankMovement`) AxisValue))

(event `InputAxis|Turn`
  (params (AxisValue :type "Float (single-precision)"))
  ;[1 1 1] Action Input Binding
  (`TankMovementComponent.IntendTurn` (`self.TankMovement`) AxisValue))

(fn `UserConstructionScript`)