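; Player-controlled tank pawn that wires its barrel, turret and tracks into TankAiming and TankMovement components on BeginPlay and caps FPS at 80.
; Input drives movement intent or per-track throttle with directional force feedback, rotates the camera gimbal and spring arm, and toggles two cameras.
; Fire calls TankAiming, then gates sound and rumble on firing state; driving sound triggers when Move input is zero.
; Widget creation, pitch clamping and older input experiments are disconnected.
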(event `self.ReceiveBeginPlay`
  (`TankAimingComponent.InitialiseAiming` (`self.TankAiming`) (`self.Barrel`) (`self.Turret`) null)
  (`TankMovementComponent.Initialise` (`self.TankMovement`) (`self.LeftTrackNew2`) (`self.RightTrackNew2`))
  (`KismetSystemLibrary.ExecuteConsoleCommand` "t.MaxFPS 80" null))

(event `self.ReceiveTick`
  (params (DeltaSeconds :type "Float (single-precision)")))

(event `InputAction|Fire`
  (params (Key :type "Key Structure"))
  ;[1 1 1] Action Input Binding
  ;;[1 1 1] Fire
  (:`Pressed`
    (`TankAimingComponent.Fire` (`self.TankAiming`))
    (if (not (select `EFiringState` (`TankAimingComponent.FiringState` (`self.TankAiming`)) :`Reloading` true :`OutOfAmmo` true))
      (`GameplayStatics.SpawnSoundAtLocation` "/Game/Vehicles/ImprovedTank/Tank_Firing_-_Post_Edit_Sound_Effect.Tank_Firing_-_Post_Edit_Sound_Effect" (`SceneComponent.K2_GetComponentLocation` (`self.Barrel`)) (struct) 1.0 1.0 0.0 "/Game/Vehicles/ImprovedTank/FireAtten.FireAtten" null)
      (`PlayerController.K2_ClientPlayForceFeedback` (`GameplayStatics.GetPlayerController` 0) "/Game/ForceFeedback/FireFeedback.FireFeedback" "None" false false false))))

(event `InputAxis|AimAzimuth`
  (params (AxisValue :type "Float (single-precision)"))
  ;[1 1 1] Camera Input Binding
  ;;[1 1 1] X Axis
  (`SceneComponent.K2_AddLocalRotation` (`self.Azimuth Gimbal`) (`KismetMathLibrary.MakeRotator` 0.0 0.0 (* AxisValue (`GameplayStatics.GetWorldDeltaSeconds`) 100.0)) false false))

(event `InputAxis|Right Track Throttle`
  (params (AxisValue :type "Float (single-precision)"))
  (bind _returnvalue (`KismetMathLibrary.FClamp` AxisValue -1.0))
  ;[1 1 1] Action Input Binding
  ;;[1 1 1] InputAxis Right Track Throttle (Axis value Connected to SetThrottle and X
  (`TankTrack.SetThrottle` (`self.RightTrackNew2`) AxisValue)
  (if (> _returnvalue 0.01)
    (`PlayerController.K2_ClientPlayForceFeedback` (`GameplayStatics.GetPlayerController` 0) "/Game/ForceFeedback/RightTrackFeedback.RightTrackFeedback" "None" false false false)
    (elif (> -0.01 _returnvalue)
      (`PlayerController.K2_ClientPlayForceFeedback` (`GameplayStatics.GetPlayerController` 0) "/Game/ForceFeedback/LeftTrackFeedback.LeftTrackFeedback" "None" false false false))))

(event `InputAxis|Left Track Throttle`
  (params (AxisValue :type "Float (single-precision)"))
  (bind _returnvalue (`KismetMathLibrary.FClamp` AxisValue -1.0))
  ;[1 1 1] Action Input Binding
  ;;[1 1 1] InputAxis Left Track Throttle (Axis value Connected to SetThrottle and X
  (`TankTrack.SetThrottle` (`self.LeftTrackNew2`) AxisValue)
  (if (> _returnvalue 0.01)
    (`PlayerController.K2_ClientPlayForceFeedback` (`GameplayStatics.GetPlayerController` 0) "/Game/ForceFeedback/LeftTrackFeedback.LeftTrackFeedback" "None" false false false)
    (elif (> -0.01 _returnvalue)
      (`PlayerController.K2_ClientPlayForceFeedback` (`GameplayStatics.GetPlayerController` 0) "/Game/ForceFeedback/RightTrackFeedback.RightTrackFeedback" "None" false false false))))

(event `InputAxis|AimElevation`
  (params (AxisValue :type "Float (single-precision)"))
  ;[1 1 1] Camera Input Binding
  ;;[1 1 1] Y Axis
  (`SceneComponent.K2_AddLocalRotation` (`self.SpringArm`) (`KismetMathLibrary.MakeRotator` 0.0 (* AxisValue (`GameplayStatics.GetWorldDeltaSeconds`) 100.0)) false false)
  (`SceneComponent.K2_AddLocalRotation` (`self.Camera1`) (`KismetMathLibrary.MakeRotator` 0.0 (* AxisValue (`GameplayStatics.GetWorldDeltaSeconds`) 100.0)) false false))

(event `InputAxis|Move`
  (params (AxisValue :type "Float (single-precision)"))
  ;[1 1 1] Action Input Binding
  ;;[1 1 1] InputAxis Move (Axis value connected to throw)
  (`TankMovementComponent.IntendMoveForward` (`self.TankMovement`) (`KismetMathLibrary.FClamp` AxisValue -1.0))
  (if (not (or (!= AxisValue 0.0) (!= (stale `InputAxis|Turn` AxisValue) 0.0)))
    (`AudioComponent.Play` (`self.DrivingSound`) 0.0)))

(event `InputAxis|Turn`
  (params (AxisValue :type "Float (single-precision)"))
  ;[1 1 1] Action Input Binding
  ;;[1 1 1] InputAxis Turn (Axis value connected to turn throw)
  (`TankMovementComponent.IntendTurn` (`self.TankMovement`) (`KismetMathLibrary.FClamp` AxisValue -1.0)))

(event `InputAction|ChangeCamera`
  (params (Key :type "Key Structure"))
  (:`Pressed`
    (`ActorComponent.ToggleActive` (`self.Camera`))
    (`ActorComponent.ToggleActive` (`self.Camera1`))))

(event `InputAxis|Move Keyboard`
  (params (AxisValue :type "Float (single-precision)"))
  ;[1 1 1] Action Input Binding
)

(event `InputAxis|Turn Keyboard`
  (params (AxisValue :type "Float (single-precision)"))
  ;[1 1 1] Action Input Binding
)

(fn `UserConstructionScript`)