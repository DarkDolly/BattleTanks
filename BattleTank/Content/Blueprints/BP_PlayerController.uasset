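; Player controller that manages the player's HUD and a gamepad pause menu.
; On begin play it creates the pause menu widget and caches the possessed broken-tank pawn.
; The FoundAimingComponent event spawns the player UI and passes it the aiming component reference.
; Pause and back-out inputs open or close the menu, switching input mode, mouse cursor and game pause state.
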(event `self.FoundAimingComponent`
  (params (AimingComponentReference :type "TankAimingComponent Object Reference"))
  (bind _returnvalue (`|CreateWidget` "/Game/Blueprints/UserInterface/PlayerUI.PlayerUI_C"))
  (set `/Game/Blueprints/UserInterface/PlayerUI.BP Aiming Component Reference` AimingComponentReference _returnvalue)
  (`UserWidget.AddToViewport` _returnvalue 0))

(event `self.ReceiveBeginPlay`
  (bind _returnvalue (`|CreateWidget` "/Game/Blueprints/UserInterface/GamePadPauseMenuUI.GamePadPauseMenuUI_C"))
  (set `self.PauseMenu` _returnvalue)
  (bind _asbp_tank_new_broken (cast `/Game/Vehicles/ImprovedTank/BP_Tank_New_Broken_Auto3` (`self.K2_GetPawn`)))
  (set `self.As BP Tank New` _asbp_tank_new_broken))

(event `InputAction|BackOut`
  (params (Key :type "Key Structure"))
  (:`Pressed`
    (`self.ClosePauseMenu`)))

(event `InputAction|PauseMenu`
  (params (Key :type "Key Structure"))
  ;[1 1 1] Pause Menu Open/Close
  (:`Pressed`
    (if (`self.PauseMenuOpened`)
      (`self.ClosePauseMenu`)
      (else
        (`self.OpenPauseMenu`)))))

(event `ClosePauseMenu`
  ;[1 1 1] Pause Menu Open/Close
  (`Widget.RemoveFromParent` (`self.PauseMenu`))
  (`WidgetBlueprintLibrary.SetInputMode_GameOnly` self)
  (set `self.bShowMouseCursor` false)
  (set `self.PauseMenuOpened` false)
  (`GameplayStatics.SetGamePaused` false))

(event `OpenPauseMenu`
  (bind _pausemenu (`self.PauseMenu`))
  ;[1 1 1] Pause Menu Open/Close
  (`UserWidget.AddToViewport` _pausemenu 0)
  (`WidgetBlueprintLibrary.SetInputMode_GameAndUIEx` self _pausemenu)
  (set `self.bShowMouseCursor` true)
  (set `self.PauseMenuOpened` true)
  (`GameplayStatics.SetGamePaused` true))

(fn `UserConstructionScript`)